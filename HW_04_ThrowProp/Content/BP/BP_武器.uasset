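; Weapon Blueprint (BP_武器) that fires bullets and tracks magazine and reserve ammo.
; The 開槍 input spawns BP_子彈 at the weapon mesh's 子彈插槽 socket while rounds remain, then decrements the magazine count.
; The 換彈匣 custom event, not called within this graph, refills the magazine from the reserve, capped by the rounds left, and deducts that amount from the total.
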(event Custom|換彈匣
  ;[0 1 0.2846] 計算要補充幾顆子彈
  (Variables|Default|Set要補充的子彈數量 (- (Variables|Default|Get彈匣尺寸) (Variables|Default|Get目前子彈數量))) ; 計算要補充的數量\n例:目前 10  彈匣 30 所以要補充20
  ;[0 1 0.2846] 判斷總是數否>=要補充數量
  (if (>= (Variables|Default|Get子彈總數) (Variables|Default|Get要補充的子彈數量))
    _
    (else
      ;[0 1 0.2846] 總數<要補充數量:把剩餘總數補充
      (Variables|Default|Set要補充的子彈數量 (Variables|Default|Get子彈總數))))
  ;[0 1 0.2846] 目前子彈以及更新總數
  (Variables|Default|Set目前子彈數量 (+ (Variables|Default|Get目前子彈數量) (Variables|Default|Get要補充的子彈數量))) ; 補充子彈數量\n例:目前 10 補充 20 補充後為 30
  (Variables|Default|Set子彈總數 (- (Variables|Default|Get子彈總數) (Variables|Default|Get要補充的子彈數量))) ; 扣除子彈總數\n例:總數為 20 要補充為 20 補充後總數為 0
)

(event Input|ActionEvents|InputAction開槍
  (params (Key :type Key%20Structure :default "None"))
  ;[1 1 1] 開槍
  (:Pressed
    (if (> (Variables|Default|Get目前子彈數量) 0) ; 當目前子彈數量大於0才能開槍
      (Game|SpawnActorfromClass "/Game/BP/BP_子彈.BP_子彈_C" (Transformation|GetSocketTransform (Variables|Default|Get武器模型) "子彈插槽" "RTS_World") "Undefined" 0 0) ; 生成子彈藍圖
      (Variables|Default|Set目前子彈數量 (- (Variables|Default|Get目前子彈數量) 1)) ; 開槍後子彈數量減一
    )))

(fn ConstructionScript)